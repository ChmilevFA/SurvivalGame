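; BP_KGProjectileBase is a projectile actor, named as a base class, that damages characters it overlaps.
; On overlap with a BP_KGCharacterBase other than its Instigator, it applies fixed damage credited to the Instigator's controller, then destroys itself.
; Overlaps with other actor types are ignored.
; The Destroyed event spawns the P_Impulse particle effect at the projectile's location, so the effect is not tied only to hits.
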(event EventBeginPlay)

(event Collision|EventActorBeginOverlap
  (params (OtherActor :type Actor%20Object%20Reference))
  (bind _instigator (Variables|Actor|GetInstigator))
  (bind _asbp_kgcharacter_base (Utilities|Casting|CastToBP_KGCharacterBase OtherActor))
  (if (not (== _asbp_kgcharacter_base _instigator))
    (Game|Damage|ApplyDamage _asbp_kgcharacter_base 5e+01 (Pawn|GetController _instigator) self)
    (Actor|DestroyActor)))

(event EventTick
  (params (DeltaSeconds :type Float%20%28single-precision%29)))

(event EventDestroyed
  (Effects|SpawnEmitteratLocation "/Game/Assets/Effects/P_Impulse.P_Impulse" (Transformation|GetActorLocation)))

(fn ConstructionScript)