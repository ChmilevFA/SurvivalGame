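; PB_KGHealthPickup is a health pickup that restores health to a BP_KGCharacterBase character that overlaps it.
; On overlap it adds HealthOffering to the character's Health, capped at the class default Health, which serves as the maximum.
; The pickup destroys itself only when it is used, so a character already at default health leaves it in place.
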(event EventBeginPlay)

(event Collision|EventActorBeginOverlap
  (params (OtherActor :type Actor%20Object%20Reference))
  (bind _asbp_kgcharacter_base (Utilities|Casting|CastToBP_KGCharacterBase OtherActor))
  (if (not (== (Variables|/Game/Blueprints/BP_KGCharacterBase.BP_KGCharacterBase_C|GetHealth _asbp_kgcharacter_base) (.Health (Utilities|GetClassDefaults (Utilities|GetClass _asbp_kgcharacter_base)))))
    (Variables|/Game/Blueprints/BP_KGCharacterBase.BP_KGCharacterBase_C|SetHealth _asbp_kgcharacter_base (Math|Float|Min(Float) (.Health (Utilities|GetClassDefaults (Utilities|GetClass _asbp_kgcharacter_base))) (+ (Variables|/Game/Blueprints/BP_KGCharacterBase.BP_KGCharacterBase_C|GetHealth _asbp_kgcharacter_base) (Variables|Default|GetHealthOffering))))
    (Actor|DestroyActor)))

(event EventTick
  (params (DeltaSeconds :type Float%20%28single-precision%29)))

(fn ConstructionScript)